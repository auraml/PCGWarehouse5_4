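; BP_PCG_Pallet_Rotation is a custom Blueprint PCG element that gives points, by its name rack pallets, a slight random yaw.
; ExecuteWithContext converts the first input's spatial data to points, runs the point loop and returns the result as a data collection.
; PointLoopBody replaces each point's yaw with a random value within a few degrees of zero, keeping location, roll, pitch and scale.
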(fn ExecutewithContext
  (params (InContext :type PCG%20Context%20Structure%20%28by%20ref%29) (Input :type PCG%20Data%20Collection%20Structure%20%28by%20ref%29))
  (bind _returnvalue (Class|PCGDataFunctionLibrary|GetInputs Input))
  (bind _aspcgspatial_data (Utilities|Casting|CastToPCGSpatialData (.Data (Utilities|Struct|BreakPCGTaggedData (Utilities|Array|Get(acopy) _returnvalue))))
    (:then
      (bind _outdata (PCG|FlowControl|PointLoop InContext (SpatialData|ToPointDatawithContext _aspcgspatial_data InContext) 0))
      (return (Utilities|Struct|MakePCGDataCollection (Utilities|Array|MakeArray (Utilities|Struct|MakePCGTaggedData _outdata 0 "None")))))
    (:CastFailed
      (return ""))))

(fn PointLoopBody
  (params (InContext :type PCG%20Context%20Structure%20%28by%20ref%29) (InData :type PCG%20Point%20Data%20Object%20Reference) (InPoint :type PCG%20Point%20Structure%20%28by%20ref%29) (OutMetadata :type PCG%20Metadata%20Object%20Reference) (Iteration :type Integer64))
  (bind _transform (Utilities|Struct|BreakPCGPoint InPoint))
  (bind _structout (Utilities|Struct|SetmembersinPCGPoint InPoint (Math|Transform|MakeTransform (.location _transform) (Math|Rotator|MakeRotator (.roll (.rotation _transform)) (.pitch (.rotation _transform)) (Math|Random|RandomFloatinRange -5.0 5.0)) (.scale _transform))))
  (return _structout true))