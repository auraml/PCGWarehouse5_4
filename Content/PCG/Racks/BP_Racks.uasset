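; BP_Racks is a procedural rack actor that builds shelves and frames through a PCG graph.
; The construction script converts shelf and frame dimensions into offset vectors on the graph instance and places the end frame from column count and shelf width.
; It derives flags and counts for additional rows, columns and frame rows, with roughly one frame row per two rack rows, then triggers local PCG generation.
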(event EventBeginPlay)

(event Collision|EventActorBeginOverlap
  (params (OtherActor :type Actor%20Object%20Reference)))

(event EventTick
  (params (DeltaSeconds :type Float%20%28single-precision%29)))

(fn ConstructionScript
  (bind _rack_rows (Variables|Rack|GetRack%20Rows))
  (bind _rack_columns (Variables|Rack|GetRack%20Columns))
  (bind _pcg (Variables|Default|GetPCG))
  (bind _shelf_dimensions (Variables|Rack|GetShelf%20Dimensions))
  (bind _frame_dimensions (Variables|Rack|GetFrame%20Dimensions))
  (bind _returnvalue (/ (.x _shelf_dimensions) 2))
  (bind _returnvalue_2 (/ (.x _frame_dimensions) 2.0))
  (bind _returnvalue_3 (+ _rack_rows 1))
  (bind _returnvalue_4 (/ (.y _frame_dimensions) 2.0))
  (bind _returnvalue_5 (/ (.y _shelf_dimensions) 2.0))
  (bind _graphinstance (Variables|/Script/PCG.PCGComponent|GetGraphInstance _pcg))
  (bind _returnvalue_6 (Math|Conversions|ToFloat(Integer) _returnvalue))
  (bind _returnvalue_7 (/ _returnvalue_3 2))
  ;[1 1 1] Shelf
  (Effects|Components|ParticleSystem|SetVectorParameter _graphinstance "ShelfOffset" (Math|Vector|MakeVector _returnvalue_6 0.0 (.z _shelf_dimensions)))
  (Effects|Components|ParticleSystem|SetVectorParameter _graphinstance "ShelfOffsetMin" (Math|Vector|MakeVector (* _returnvalue_6 -1) (* _returnvalue_5 -1.0) (* (.z _shelf_dimensions) -1.0)))
  (Effects|Components|ParticleSystem|SetVectorParameter _graphinstance "ShelfOffsetMax" (Math|Vector|MakeVector _returnvalue_6 _returnvalue_5 0.0))
  ;[1 1 1] Frame
  (Effects|Components|ParticleSystem|SetVectorParameter _graphinstance "FrameOffsetMin" (Math|Vector|MakeVector (* _returnvalue_2 -1.0) (* _returnvalue_4 -1.0) 0.0))
  (Effects|Components|ParticleSystem|SetVectorParameter _graphinstance "FrameOffsetMax" (Math|Vector|MakeVector _returnvalue_2 _returnvalue_4 (.z _frame_dimensions)))
  ;[1 1 1] Set Additinal Rows and Colums Variables
  (Variables|Rack|SetMultiple%20Rows (> _rack_rows 1))
  (Variables|Rack|SetAdditional%20Rows (- _rack_rows 1))
  (Variables|Rack|SetMultiple%20Columns (> _rack_columns 1))
  (Variables|Rack|SetAdditional%20Columns (- _rack_columns 1))
  (Variables|Rack|SetMultiple%20Frame%20Rows (>= _returnvalue_7 2))
  (Variables|Rack|SetAdditional%20Frame%20Rows (- _returnvalue_7 1))
  ;[1 1 1] End Frame
  (Effects|Components|ParticleSystem|SetVectorParameter _graphinstance "EndFrameTransform" (Math|Vector|MakeVector (* (Variables|Rack|GetRack%20Columns) (.x (Variables|Rack|GetShelf%20Dimensions))) 0.0 0.0))
  (Class|PCGComponent|GenerateLocal (Variables|Default|GetPCG) false))